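; Base enemy AI controller that routes perception updates to sight, hearing and damage responses.
; On each update it checks every changed actor against all three senses, passing the actor to the sight and damage handlers and the stimulus location to the sound handler.
; Hearing uses a local CanSenseActorBP helper that matches last sensed stimuli by sense class to expose the stimulus; the other checks and all handlers are defined outside this graph.
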(event OnPerceptionUpdated(AIPerceptionComponent)
  (params (UpdatedActors :type Array%20of%20Actor%20Object%20References))
  (for _array_element UpdatedActors
    (Utilities|FlowControl|Sequence
      (:then_0
        (bind _returnvalue (Class|AICEnemyBase|CanSenseActor _array_element "EAS_Sight"))
        (if _returnvalue
          (Class|AICEnemyBase|HandleSensedSight _array_element)))
      (:then_1
        (bind (_sensed _stimulus) (CallFunction|CanSenseActorBP _array_element "EAS_Hearing"))
        (if _sensed
          (Class|AICEnemyBase|HandleSensedSound (.StimulusLocation (Utilities|Struct|BreakAIStimulus _stimulus)))))
      (:then_2
        (bind _returnvalue_2 (Class|AICEnemyBase|CanSenseActor _array_element "EAS_Damage"))
        (if _returnvalue_2
          (Class|AICEnemyBase|HandleSensedDamage _array_element))))))

(fn ConstructionScript)

(fn CanSenseActorBP
  (params (Actor :type Actor%20Object%20Reference) (Sense :type EAISense%20Enum :default "EAS_None"))
  (bind _info (Class|AIPerceptionComponent|GetActorsPerception (Variables|Default|GetAIPerceptionComponent) Actor))
  (for _array_element (.LastSensedStimuli (Utilities|Struct|BreakActorPerceptionBlueprintInfo _info))
    (bind _returnvalue (Class|AIPerceptionSystem|GetSenseClassforStimulus _array_element))
    (if (== _returnvalue (Utilities|Select :Index Sense :EAS_None 0 :EAS_Sight "/Script/AIModule.AISense_Sight" :EAS_Hearing "/Script/AIModule.AISense_Hearing" :EAS_Damage "/Script/AIModule.AISense_Damage"))
      (return (.bSuccessfullySensed (Utilities|Struct|BreakAIStimulus _array_element)) _array_element))))