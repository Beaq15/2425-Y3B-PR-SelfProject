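; Base enemy character that handles sword combat animations, exposes a patrol route and switches movement speed.
; Attack plays a great sword slash montage and fires OnAttackEnd on completion or interruption.
; WieldSword and DropSword use montage notifies to spawn and socket-attach or destroy BP_Sword, firing their dispatchers only on completion.
; SetMovementSpeed maps a gait enum from Idle to Sprinting onto MaxWalkSpeed and returns it.
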(event Custom|Attack
  (Animation|Montage|PlayMontage (Variables|Character|GetMesh) "/Game/Enemies/Great_Sword_Slash_mixamo_com1_Montage.Great_Sword_Slash_mixamo_com1_Montage"
    (:OnCompleted
      _)
    (:OnInterrupted
      _))
  (Default|CallOnAttackEnd))

(event Custom|WieldSword
  (bind _notifyname (Animation|Montage|PlayMontage (Variables|Character|GetMesh) "/Game/Enemies/Show_Sword_Montage.Show_Sword_Montage")
    (:OnCompleted
      (Default|CallOnWieldSword))
    (:OnNotifyBegin
      (switch name _notifyname
        (:ShowSword
          (bind _returnvalue (Game|SpawnActorfromClass "/Game/Weapons/BP_Sword.BP_Sword_C" (Transformation|GetActorTransform) "Undefined" "MultiplyWithRoot" 0 0))
          (bind _output_get (Variables|Default|SetSwordActor _returnvalue))
          (Transformation|AttachComponentToComponent _output_get (Variables|Character|GetMesh) "hand_r_sword_socket" "SnapToTarget" "SnapToTarget" "SnapToTarget" true)
          (Variables|Default|SetIsWieldingSword true))))))

(event Custom|DropSword
  (bind _notifyname (Animation|Montage|PlayMontage (Variables|Character|GetMesh) "/Game/Enemies/Hide_Sword_Montage.Hide_Sword_Montage")
    (:OnCompleted
      (Default|CallOnDropSword))
    (:OnNotifyBegin
      (switch name _notifyname
        (:DropSword
          (Actor|DestroyActor (Variables|Default|GetSwordActor))
          (Variables|Default|SetIsWieldingSword false))))))

(event EventBeginPlay)

(fn ConstructionScript)

(fn GetPatrolRoute
  (return (Variables|AI|GetPatrolRoute)))

(fn SetMovementSpeed
  (params (Speed :type E_MovementSpeed%20Enum :default "NewEnumerator0"))
  (bind _output_get (Variables|/Script/Engine.CharacterMovementComponent|SetMaxWalkSpeed (Variables|Character|GetCharacterMovement) (Utilities|Select :Index Speed :NewEnumerator0 0.0 :NewEnumerator1 1e+02 :NewEnumerator2 3e+02 :NewEnumerator3 5e+02)))
  (return _output_get))